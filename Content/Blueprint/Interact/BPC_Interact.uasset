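; Interaction component that lets a character trigger items in front of the follow camera.
; InteractWithItem runs a sphere trace forward from the camera on a dedicated trace channel, storing any hit actor that implements BPI_Interact.
; It then sends InteractMessage to the stored item, which is not cleared on a miss, so the last found item stays targeted.
; Initialization supplies the owning character reference.
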(event `InteractWithItem`
  (`self.FindInteractableItem`)
  (bind _interactableitem (`self.InteractableItem`)
    (:`then`
      (message `/Game/Blueprint/Interact/BPI_Interact.Interact` _interactableitem))
    (:`else`)))

(fn `FindInteractableItem`
  (bind _followcamera (`/Game/OtherAssets/ThirdPersonBP/Blueprints/ThirdPersonCharacter.FollowCamera` (`self.Character`)))
  (bind _returnvalue (`SceneComponent.K2_GetComponentLocation` _followcamera))
  (bind _outhit (`KismetSystemLibrary.SphereTraceSingle` _returnvalue (+ _returnvalue (* (`SceneComponent.GetForwardVector` _followcamera) 1000.0)) 100.0 "TraceTypeQuery3"))
  (bind (_bblockinghit _binitialoverlap _time _distance _location _impactpoint _normal _impactnormal _physmat _hitactor) (`GameplayStatics.BreakHitResult` _outhit))
  (if (`KismetSystemLibrary.DoesImplementInterface` _hitactor "/Game/Blueprint/Interact/BPI_Interact.BPI_Interact_C")
    (set `self.InteractableItem` _hitactor)))

(fn `Initialization`
  (params (Character :type "/Game/OtherAssets/ThirdPersonBP/Blueprints/ThirdPersonCharacter Object Reference"))
  (set `self.Character` Character))
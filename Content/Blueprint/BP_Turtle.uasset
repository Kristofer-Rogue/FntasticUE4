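; BP_Turtle is an AI-driven turtle actor that hands its start and finish positions to its Blackboard.
; On BeginPlay it writes both positions as object values under key names held in variables.
; The construction script assigns the AI controller class from a variable of the same name.
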(event `self.ReceiveBeginPlay`
  (set `self.Blackboard` (`AIBlueprintHelperLibrary.GetBlackboard` self))
  (`BlackboardComponent.SetValueAsObject` (`self.Blackboard`) (`self.StartPositionName`) (`self.StartPosition`))
  (`BlackboardComponent.SetValueAsObject` (`self.Blackboard`) (`self.FinishPositionName`) (`self.FinishPosition`)))

(fn `UserConstructionScript`
  (set `self.AIControllerClass` (`self.AI Controller Class`)))